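; BP_PrimeTest is a trigger Blueprint that runs a prime-finding task when a Character overlaps its collider, likely to compare main-thread and background-thread execution.
; A flag chooses between running the task on the main thread or on a background thread.
; A Ready gate blocks re-triggering until the synchronous call returns or the OnDoneFindingPrimes event fires and prints a message.
; Ready clears before the Character cast, so a non-Character overlap leaves it locked.
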(event `self.Collide.OnComponentBeginOverlap`
  (params (OverlappedComponent :type "PrimitiveComponent Object Reference") (OtherActor :type "Actor Object Reference") (OtherComp :type "PrimitiveComponent Object Reference") (OtherBodyIndex :type Integer) (bFromSweep :type Boolean) (SweepResult :type "HitResult Structure (by ref)"))
  (bind _numprimestofind (`self.NumPrimesToFind`))
  (if (`self.Ready`)
    (set `self.Ready` false)
    (cast `Character` OtherActor)
    (if (`self.RunOnMainThread?`)
      (`self.RunPrimeTaskOnMainThread` _numprimestofind)
      (set `self.Ready` true)
      (else
        (`self.RunPrimeTaskOnBackgroundThread` _numprimestofind)))))

(event `self.OnDoneFindingPrimes`
  (`KismetSystemLibrary.PrintString` "Done Finding Primes (blueprint)")
  (set `self.Ready` true))

(fn `UserConstructionScript`)